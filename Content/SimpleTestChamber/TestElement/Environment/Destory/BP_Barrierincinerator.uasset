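; BP_Barrierincinerator is a test-chamber barrier that visually reacts to objects entering it, with two optional border lights.
; Overlap on either trigger box restarts a timeline that lerps the Cube material's transparency; no destruction logic appears here.
; ButtonActive and ButtonDeactive play or reverse a timeline blending both lights' emissive color.
; The construction script sets initial transparency, border visibility and collision from Hasborder, and light color from IsActive.
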(event OnComponentBeginOverlap(DestoryTriggerBox)
  (params (OverlappedComponent :type Primitive%20Component%20Object%20Reference) (OtherActor :type Actor%20Object%20Reference) (OtherComp :type Primitive%20Component%20Object%20Reference) (OtherBodyIndex :type Integer) (bFromSweep :type Boolean) (SweepResult :type Hit%20Result%20Structure%20%28by%20ref%29))
  (bind _lerp (Timeline|DestroyAnim PlayFromStart)
    (:Update
      (Rendering|Material|SetScalarParameterValueonMaterials (Variables|Default|GetCube) "transparent" (Math|Float|Lerp (Variables|Default|GetMin_transparent) (Variables|Default|GetMax_transparent) _lerp)))))

(event OnComponentBeginOverlap(PhyDestoryTriggerBox)
  (params (OverlappedComponent :type Primitive%20Component%20Object%20Reference) (OtherActor :type Actor%20Object%20Reference) (OtherComp :type Primitive%20Component%20Object%20Reference) (OtherBodyIndex :type Integer) (bFromSweep :type Boolean) (SweepResult :type Hit%20Result%20Structure%20%28by%20ref%29))
  (bind _lerp (Timeline|DestroyAnim PlayFromStart)
    (:Update
      (Rendering|Material|SetScalarParameterValueonMaterials (Variables|Default|GetCube) "transparent" (Math|Float|Lerp (Variables|Default|GetMin_transparent) (Variables|Default|GetMax_transparent) _lerp)))))

(event EventButtonDeactive
  (bind _lerp (Timeline|Animation_0 Reverse)
    (:Update
      (CallFunction|LerponMaterialColor (Variables|Default|GetLight2) "EmissiveColor" (Variables|Default|GetColorA) (Variables|Default|GetColorB) _lerp)
      (CallFunction|LerponMaterialColor (Variables|Default|GetLight1) "EmissiveColor" (Variables|Default|GetColorA) (Variables|Default|GetColorB) _lerp))))

(event EventButtonActive
  (bind _lerp (Timeline|Animation_0 Play)
    (:Update
      (CallFunction|LerponMaterialColor (Variables|Default|GetLight2) "EmissiveColor" (Variables|Default|GetColorA) (Variables|Default|GetColorB) _lerp)
      (CallFunction|LerponMaterialColor (Variables|Default|GetLight1) "EmissiveColor" (Variables|Default|GetColorA) (Variables|Default|GetColorB) _lerp))))

(fn ConstructionScript
  (bind _light2 (Variables|Default|GetLight2))
  (bind _hasborder (Variables|Default|GetHasborder))
  (Rendering|Material|SetScalarParameterValueonMaterials (Variables|Default|GetCube) "transparent" (Variables|Default|GetMin_transparent))
  (Rendering|SetVisibility (Variables|Default|GetLight1) _hasborder false)
  (Collision|SetCollisionEnabled _light2 (select _hasborder "PhysicsOnly" "NoCollision"))
  (Rendering|Material|SetColorParameterValueonMaterials _light2 "EmissiveColor" (select (Variables|Default|GetIsActive) (Variables|Default|GetColorB) (Variables|Default|GetColorA))))