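; BP_Light is a placeable test-chamber light that can be switched by a linked event target, letting many lights follow one trigger.
; Construction applies its initial lit state and color to the point and rect lights.
; BeginPlay binds ButtonActive to the target; ButtonDeactive switches it off but is not bound here.
; Switching toggles RectLight visibility, propagated to children, and the Cube material's intensity parameter to match.
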(event EventBeginPlay
  (bind _eventtarget (Variables|Default|GetEventTarget))
  ;[0.15 0.15 0.15 0.5] ThisBPHasAEventDispatcherSoYouCanLotsOfLightsLinkWithADoorWithEase
  (Utilities|IsValid _eventtarget
    (:Is%20Valid
      (EventDispatchers|BindEventtoActive _eventtarget (delegate EventButtonActive)))))

(event EventButtonActive
  ;[0.15 0.15 0.15 0.5] ThisBPHasAEventDispatcherSoYouCanLotsOfLightsLinkWithADoorWithEase
  (CallFunction|SetLightActive true))

(event EventButtonDeactive
  ;[0.15 0.15 0.15 0.5] ThisBPHasAEventDispatcherSoYouCanLotsOfLightsLinkWithADoorWithEase
  (CallFunction|SetLightActive false))

(fn ConstructionScript
  (|CallParentFunction)
  (CallFunction|SetLightActive (Variables|Default|GetIsLit))
  (CallFunction|SetLightColor (Variables|Default|GetLightColor)))

(fn SetLightActive
  (params (IsActive :type Boolean))
  (bind _output_get (LocalVariables|SetIsActiveLoc IsActive))
  (Rendering|SetVisibility (Variables|Default|GetRectLight) _output_get true)
  (Rendering|Material|SetScalarParameterValueonMaterials (Variables|Default|GetCube) "intensity" (Math|Float|SelectFloat 1.0 0.0 _output_get)))

(fn SetLightColor
  (params (NewLightColor :type Linear%20Color%20Structure))
  (Rendering|Components|Light|SetLightColor (Variables|Default|GetPointLight) NewLightColor true)
  (Rendering|Components|Light|SetLightColor (Variables|Default|GetRectLight) NewLightColor true))