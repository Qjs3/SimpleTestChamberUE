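; Springboard test element that, while switched on by button events, launches the player or physics objects along an arc to a Billboard target.
; Separate triggers compute the custom-arc velocity: one calls LaunchCharacter, the other releases the player's grab and overrides physics velocity.
; A timeline fades material opacity and emissive color with the on state, which the construction script mirrors.
; Tick draws the predicted arc when ShowArc is set, as happens when BeginPlay finds no player character.
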(event OnComponentBeginOverlap(PlayerTriggler)
  (params (OverlappedComponent :type Primitive%20Component%20Object%20Reference) (OtherActor :type Actor%20Object%20Reference) (OtherComp :type Primitive%20Component%20Object%20Reference) (OtherBodyIndex :type Integer) (bFromSweep :type Boolean) (SweepResult :type Hit%20Result%20Structure%20%28by%20ref%29))
  (if (Variables|Default|GetIsOn)
    (Variables|Default|SetOther%20Actor OtherActor)
    (bind _asbp_first_person_character (Utilities|Casting|CastToBP_FirstPersonCharacter (Variables|Default|GetOther%20Actor)))
    (bind _output_get (Variables|Default|SetAs%20BP%20First%20Person%20Character _asbp_first_person_character))
    (bind _outlaunchvelocity (Game|SuggestProjectileVelocityCustomArc (Transformation|GetActorLocation _output_get) (Transformation|GetWorldLocation (Variables|Default|GetBillboard)) 0.0 (Variables|Default|GetArc%20Param)))
    (Character|LaunchCharacter (Variables|Default|GetAs%20BP%20First%20Person%20Character) _outlaunchvelocity true true)))

(event OnComponentBeginOverlap(PhyTriggler)
  (params (OverlappedComponent :type Primitive%20Component%20Object%20Reference) (OtherActor :type Actor%20Object%20Reference) (OtherComp :type Primitive%20Component%20Object%20Reference) (OtherBodyIndex :type Integer) (bFromSweep :type Boolean) (SweepResult :type Hit%20Result%20Structure%20%28by%20ref%29))
  (if (Variables|Default|GetIsOn)
    (bind _asbp_first_person_character (Utilities|Casting|CastToBP_FirstPersonCharacter (Game|Player|GetPlayerPawn 0)))
    (Default|ReleaseGrab _asbp_first_person_character)
    (bind _output_get (Variables|Default|SetOther%20CompPhy OtherComp))
    (bind _outlaunchvelocity (Game|SuggestProjectileVelocityCustomArc (Transformation|GetWorldLocation _output_get) (Transformation|GetWorldLocation (Variables|Default|GetBillboard)) 0.0 (Variables|Default|GetArc%20Param)))
    (Class|PrimitiveComponent|SetAllPhysicsLinearVelocity (Variables|Default|GetOther%20CompPhy) _outlaunchvelocity false)))

(event EventBeginPlay
  (Utilities|IsValid (Game|GetPlayerCharacter 0)
    (:Is%20Not%20Valid
      (Variables|Default|SetShowArc true))))

(event EventButtonActive
  (Development|PrintString "Hello")
  (Variables|Default|SetIsOn true)
  (bind _lerp (Timeline|ActiveAnim Play)
    (:Update
      (CallFunction|LerponMaterialScalar (Variables|Default|GetEMesh) "opacity" 0.0 0.6 _lerp)
      (CallFunction|LerponMaterialColor (Variables|Default|GetPlateMesh) "EmissiveColor" (Variables|Default|GetColorA) (Variables|Default|GetColorB) _lerp))))

(event EventTick
  (params (DeltaSeconds :type Float%20%28single-precision%29))
  (if (Variables|Default|GetShowArc)
    (bind _outlaunchvelocity (Game|SuggestProjectileVelocityCustomArc (Transformation|GetWorldLocation (Variables|Default|GetBaseMesh)) (Transformation|GetWorldLocation (Variables|Default|GetBillboard)) 0.0 (Variables|Default|GetArc%20Param)))
    (Class|GameplayStatics|BlueprintPredictProjectilePathbyTraceChannel (Transformation|GetWorldLocation (Variables|Default|GetBaseMesh)) _outlaunchvelocity false 1e+01 "ECC_WorldStatic" false 0 "ForOneFrame" 0.0 15.0 5.0)))

(event EventButtonDeactive
  (Variables|Default|SetIsOn false)
  (bind _lerp (Timeline|ActiveAnim Reverse)
    (:Update
      (CallFunction|LerponMaterialScalar (Variables|Default|GetEMesh) "opacity" 0.0 0.6 _lerp)
      (CallFunction|LerponMaterialColor (Variables|Default|GetPlateMesh) "EmissiveColor" (Variables|Default|GetColorA) (Variables|Default|GetColorB) _lerp))))

(fn ConstructionScript
  (|CallParentFunction)
  (Rendering|Material|SetScalarParameterValueonMaterials (Variables|Default|GetEMesh) "opacity" (select (Variables|Default|GetIsOn) 0.6 0.0))
  (Rendering|Material|SetColorParameterValueonMaterials (Variables|Default|GetPlateMesh) "EmissiveColor" (select (Variables|Default|GetIsOn) (Variables|Default|GetColorB) (Variables|Default|GetColorA))))