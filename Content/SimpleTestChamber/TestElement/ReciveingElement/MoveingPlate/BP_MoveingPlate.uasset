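; Moving plate for a test chamber that travels along a spline, started automatically or by button activation.
; A button either moves it at once or arms it, letting Tick start movement while its box is overlapped.
; A timeline scaled by Time drives position, with options to loop, stop or reverse on deactivation or overlap end.
; A second timeline fades the ring's emissive color with movement.
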(event OnComponentBeginOverlap(Box)
  (params (OverlappedComponent :type Primitive%20Component%20Object%20Reference) (OtherActor :type Actor%20Object%20Reference) (OtherComp :type Primitive%20Component%20Object%20Reference) (OtherBodyIndex :type Integer) (bFromSweep :type Boolean) (SweepResult :type Hit%20Result%20Structure%20%28by%20ref%29))
  (Variables|Default|SetIsOverlaping true))

(event OnComponentEndOverlap(Box)
  (params (OverlappedComponent :type Primitive%20Component%20Object%20Reference) (OtherActor :type Actor%20Object%20Reference) (OtherComp :type Primitive%20Component%20Object%20Reference) (OtherBodyIndex :type Integer))
  (Variables|Default|SetIsOverlaping false)
  (if (Variables|Default|GetCanMoveNow)
    (switch Utilities|FlowControl|Switch|SwitchonE_WhenPlayerLeave (Variables|Default|GetWhenPlayerLeave)
      (:NewEnumerator1
        (CallFunction|Reverse))
      (:NewEnumerator2
        (CallFunction|Stop)))))

(event Custom|Move
  (Variables|Default|SetAnimationPlayType "NewEnumerator0")
  (CallFunction|PlayAnim)
  (Components|Timeline|SetPlayRate (Variables|Default|GetT_Move) (/ 1.0 (Variables|Default|GetTime)))
  (bind _lerp (Timeline|T_Move Play)
    (:Update
      (Transformation|SetWorldLocationAndRotation (Variables|Default|GetPlateMesh) (Spline|GetLocationatDistanceAlongSpline (Variables|Default|GetSpline) (Math|Float|Lerp 0.0 (Spline|GetSplineLength (Variables|Default|GetSpline)) _lerp) "World") "0, 0, 0" false false))
    (:Finished
      (Variables|Default|SetAnimationPlayType "NewEnumerator2")
      (Utilities|FlowControl|DoOnce false
        (:Completed
          (CallFunction|Loop))))))

(event Custom|Reverse
  (Variables|Default|SetAnimationPlayType "NewEnumerator1")
  (CallFunction|ReverseAnim)
  (bind _lerp (Timeline|T_Move Reverse)
    (:Update
      (Transformation|SetWorldLocationAndRotation (Variables|Default|GetPlateMesh) (Spline|GetLocationatDistanceAlongSpline (Variables|Default|GetSpline) (Math|Float|Lerp 0.0 (Spline|GetSplineLength (Variables|Default|GetSpline)) _lerp) "World") "0, 0, 0" false false))
    (:Finished
      (Variables|Default|SetAnimationPlayType "NewEnumerator2")
      (Utilities|FlowControl|DoOnce false
        (:Completed
          (CallFunction|Loop))))))

(event Custom|Stop
  (Variables|Default|SetAnimationPlayType "NewEnumerator2")
  (CallFunction|ReverseAnim)
  (bind _lerp (Timeline|T_Move Stop)
    (:Update
      (Transformation|SetWorldLocationAndRotation (Variables|Default|GetPlateMesh) (Spline|GetLocationatDistanceAlongSpline (Variables|Default|GetSpline) (Math|Float|Lerp 0.0 (Spline|GetSplineLength (Variables|Default|GetSpline)) _lerp) "World") "0, 0, 0" false false))
    (:Finished
      (Variables|Default|SetAnimationPlayType "NewEnumerator2")
      (Utilities|FlowControl|DoOnce false
        (:Completed
          (CallFunction|Loop))))))

(event Custom|Loop
  (if (Variables|Default|GetLoop?)
    (CallFunction|Reverse)
    (Utilities|FlowControl|Delay (Variables|Default|GetTime))
    (CallFunction|Move)
    (CallFunction|ResetLoop)))

(event Custom|ResetLoop
  (Utilities|FlowControl|DoOnce false) ; enters at Reset
)

(event EventButtonActive
  (if (Variables|Default|GetMoveWithPlayer)
    (CallFunction|Move)
    (else
      (Variables|Default|SetCanMoveNow true))))

(event EventTick
  (params (DeltaSeconds :type Float%20%28single-precision%29))
  (CallFunction|Tick 0.0))

(event EventButtonDeactive
  (Variables|Default|SetCanMoveNow false)
  (if (Variables|Default|GetStopWhenDeactive?)
    (CallFunction|Stop)
    (else
      (CallFunction|Reverse))))

(event EventBeginPlay
  (if (Variables|Default|GetAutoMove)
    (CallFunction|Move)))

(event Custom|PlayAnim
  (bind _lerp (Timeline|Anim Play)
    (:Update
      (CallFunction|LerponMaterialColor (Variables|Default|GetPlateRing) "EmissiveColor" (Variables|Default|GetA) (Variables|Default|GetB) _lerp))))

(event Custom|ReverseAnim
  (bind _lerp (Timeline|Anim Reverse)
    (:Update
      (CallFunction|LerponMaterialColor (Variables|Default|GetPlateRing) "EmissiveColor" (Variables|Default|GetA) (Variables|Default|GetB) _lerp))))

(fn ConstructionScript)

(fn Tick
  (params (Delta%20Seconds :type Float%20%28double-precision%29))
  (LocalVariables|SetNewLocalVar Delta%20Seconds)
  (Utilities|FlowControl|Sequence
    (:then_0
      (if (Math|Boolean|ANDBoolean (Variables|Default|GetCanMoveNow) (Variables|Default|GetIsOverlaping) (not (Variables|Default|GetAutoMove)))
        (CallFunction|Move)))))