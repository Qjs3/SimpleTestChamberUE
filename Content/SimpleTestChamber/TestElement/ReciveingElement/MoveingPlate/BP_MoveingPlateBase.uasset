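; Base moving plate for test chambers, carrying a mesh along a spline path when played, with stop and reverse controls.
; A timeline, rate-scaled by Time, maps its alpha to distance along the spline and calls an empty Finish event on completion.
; A second timeline blends the ring's emissive color forward or back.
; Box overlaps set an overlap flag, while the block trigger teleports entering actors to TeleportLocation.
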(event OnComponentBeginOverlap(Box)
  (params (OverlappedComponent :type Primitive%20Component%20Object%20Reference) (OtherActor :type Actor%20Object%20Reference) (OtherComp :type Primitive%20Component%20Object%20Reference) (OtherBodyIndex :type Integer) (bFromSweep :type Boolean) (SweepResult :type Hit%20Result%20Structure%20%28by%20ref%29))
  (Variables|Default|SetIsOverlaping true))

(event OnComponentEndOverlap(Box)
  (params (OverlappedComponent :type Primitive%20Component%20Object%20Reference) (OtherActor :type Actor%20Object%20Reference) (OtherComp :type Primitive%20Component%20Object%20Reference) (OtherBodyIndex :type Integer))
  (Variables|Default|SetIsOverlaping false))

(event OnComponentBeginOverlap(BlockTriggerBox)
  (params (OverlappedComponent :type Primitive%20Component%20Object%20Reference) (OtherActor :type Actor%20Object%20Reference) (OtherComp :type Primitive%20Component%20Object%20Reference) (OtherBodyIndex :type Integer) (bFromSweep :type Boolean) (SweepResult :type Hit%20Result%20Structure%20%28by%20ref%29))
  (Transformation|SetActorLocation OtherActor (Transformation|GetWorldLocation (Variables|Default|GetTeleportLocation)) false false))

(event Custom|Play
  (Components|Timeline|SetPlayRate (Variables|Default|GetT_Move) (/ 1.0 (Variables|Default|GetTime)))
  (bind (_direction _lerp) (Timeline|T_Move Play)
    (:Update
      (Variables|Default|SetT_MoveDirection _direction)
      (Transformation|SetWorldLocationAndRotation (Variables|Default|GetPlateMesh) (Spline|GetLocationatDistanceAlongSpline (Variables|Default|GetSpline) (Math|Float|Lerp 0.0 (Spline|GetSplineLength (Variables|Default|GetSpline)) _lerp) "World") "0, 0, 0" false false))
    (:Finished
      (CallFunction|Finish))))

(event Custom|Reverse
  (bind (_direction _lerp) (Timeline|T_Move Reverse)
    (:Update
      (Variables|Default|SetT_MoveDirection _direction)
      (Transformation|SetWorldLocationAndRotation (Variables|Default|GetPlateMesh) (Spline|GetLocationatDistanceAlongSpline (Variables|Default|GetSpline) (Math|Float|Lerp 0.0 (Spline|GetSplineLength (Variables|Default|GetSpline)) _lerp) "World") "0, 0, 0" false false))
    (:Finished
      (CallFunction|Finish))))

(event Custom|Stop
  (bind (_direction _lerp) (Timeline|T_Move Stop)
    (:Update
      (Variables|Default|SetT_MoveDirection _direction)
      (Transformation|SetWorldLocationAndRotation (Variables|Default|GetPlateMesh) (Spline|GetLocationatDistanceAlongSpline (Variables|Default|GetSpline) (Math|Float|Lerp 0.0 (Spline|GetSplineLength (Variables|Default|GetSpline)) _lerp) "World") "0, 0, 0" false false))
    (:Finished
      (CallFunction|Finish))))

(event Custom|finish)

(event EventBeginPlay
  (Components|Timeline|SetPlayRate (Variables|Default|GetT_Move) (/ 1.0 (Variables|Default|GetTime))))

(event Custom|PlayAnim
  (bind _lerp (Timeline|Anim Play)
    (:Update
      (CallFunction|LerponMaterialColor (Variables|Default|GetPlateRing) "EmissiveColor" (Variables|Default|GetA) (Variables|Default|GetB) _lerp))))

(event Custom|ReverseAnim
  (bind _lerp (Timeline|Anim Reverse)
    (:Update
      (CallFunction|LerponMaterialColor (Variables|Default|GetPlateRing) "EmissiveColor" (Variables|Default|GetA) (Variables|Default|GetB) _lerp))))

(fn ConstructionScript)