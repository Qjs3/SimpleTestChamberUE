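; Base sliding door for test chambers, openable by activation events or an optional auto-open trigger, with three optional auto-close triggers.
; One timeline, played forward or reversed, drives door position and light colour, while a blocking box toggles collision.
; An optional incinerator barrier spawned at BeginPlay destroys objects only while the door is open.
; The construction script configures trigger responses, exit sign and lights; auto-opening also calls delayed activation on the door target.
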(event OnComponentBeginOverlap(AutoOpenTriggerBox)
  (params (OverlappedComponent :type Primitive%20Component%20Object%20Reference) (OtherActor :type Actor%20Object%20Reference) (OtherComp :type Primitive%20Component%20Object%20Reference) (OtherBodyIndex :type Integer) (bFromSweep :type Boolean) (SweepResult :type Hit%20Result%20Structure%20%28by%20ref%29))
  ;[0.15 0.15 0.15 0.5] AutoOpen
  (if (not (Variables|Default|GetIsOpen))
    (CallFunction|ButtonActive)
    (Utilities|FlowControl|Delay (Variables|Default|GetActiveDuration))
    (Default|CallActive)
    (CallFunction|ActiveLoop (Variables|Default|GetDoorTarget))))

(event Custom|OnAutoCloseTriggleBoxActive
  ;[0.15 0.15 0.15 0.5] AutoClose
  (if (Variables|Default|GetIsOpen)
    (CallFunction|ButtonDeactive)))

(event EventButtonDeactive
  ;[0.15 0.15 0.15 0.5] Door open and close
  (Variables|Default|SetIsOpen false)
  ;;[0.15 0.15 0.15 0.5] set the invisible box collision
  (Collision|SetCollisionEnabled (Variables|Default|GetBlockingBox) "QueryAndPhysics")
  (CallFunction|SetBarrierincineratorCanDestroyObject false)
  ;;[0.15 0.15 0.15 0.5] Animation
  (bind _alpha (Timeline|OpenAnim Reverse)
    (:Update
      (CallFunction|LerponSetLocation (Variables|Default|GetDoorMain) (Variables|Default|GetDoorStartLocation) (Variables|Default|GetDoorEndLocation) _alpha)
      (CallFunction|LerponMaterialColor (Variables|Default|GetDoorLight2) "EmissiveColor" (Variables|Default|GetColorA) (Variables|Default|GetColorB) _alpha)
      (CallFunction|LerponMaterialColor (Variables|Default|GetDoorLight1) "EmissiveColor" (Variables|Default|GetColorA) (Variables|Default|GetColorB) _alpha))))

(event EventButtonActive
  ;[0.15 0.15 0.15 0.5] Door open and close
  (Variables|Default|SetIsOpen true)
  ;;[0.15 0.15 0.15 0.5] set the invisible box collision
  (Collision|SetCollisionEnabled (Variables|Default|GetBlockingBox) "NoCollision")
  (CallFunction|SetBarrierincineratorCanDestroyObject true)
  ;;[0.15 0.15 0.15 0.5] Animation
  (bind _alpha (Timeline|OpenAnim Play)
    (:Update
      (CallFunction|LerponSetLocation (Variables|Default|GetDoorMain) (Variables|Default|GetDoorStartLocation) (Variables|Default|GetDoorEndLocation) _alpha)
      (CallFunction|LerponMaterialColor (Variables|Default|GetDoorLight2) "EmissiveColor" (Variables|Default|GetColorA) (Variables|Default|GetColorB) _alpha)
      (CallFunction|LerponMaterialColor (Variables|Default|GetDoorLight1) "EmissiveColor" (Variables|Default|GetColorA) (Variables|Default|GetColorB) _alpha))))

(event OnComponentBeginOverlap(AutoCloseTriggerBox)
  (params (OverlappedComponent :type Primitive%20Component%20Object%20Reference) (OtherActor :type Actor%20Object%20Reference) (OtherComp :type Primitive%20Component%20Object%20Reference) (OtherBodyIndex :type Integer) (bFromSweep :type Boolean) (SweepResult :type Hit%20Result%20Structure%20%28by%20ref%29))
  ;[0.15 0.15 0.15 0.5] Three Auto trigger box
  (CallFunction|OnAutoCloseTriggleBoxActive))

(event OnComponentBeginOverlap(AutoCloseTriggerBox2)
  (params (OverlappedComponent :type Primitive%20Component%20Object%20Reference) (OtherActor :type Actor%20Object%20Reference) (OtherComp :type Primitive%20Component%20Object%20Reference) (OtherBodyIndex :type Integer) (bFromSweep :type Boolean) (SweepResult :type Hit%20Result%20Structure%20%28by%20ref%29))
  ;[0.15 0.15 0.15 0.5] Three Auto trigger box
  (CallFunction|OnAutoCloseTriggleBoxActive))

(event OnComponentBeginOverlap(AutoCloseTriggerBox1)
  (params (OverlappedComponent :type Primitive%20Component%20Object%20Reference) (OtherActor :type Actor%20Object%20Reference) (OtherComp :type Primitive%20Component%20Object%20Reference) (OtherBodyIndex :type Integer) (bFromSweep :type Boolean) (SweepResult :type Hit%20Result%20Structure%20%28by%20ref%29))
  ;[0.15 0.15 0.15 0.5] Three Auto trigger box
  (CallFunction|OnAutoCloseTriggleBoxActive))

(event EventBeginPlay
  (if (Variables|Default|GetHasBarrier?)
    (bind _returnvalue (Game|SpawnActorfromClass "/Game/SimpleTestChamber/TestElement/Environment/Destory/BP_Barrierincinerator.BP_Barrierincinerator_C" (Transformation|GetWorldTransform (Variables|Default|GetBarrierSpawnLocation)) "AlwaysSpawn" "OverrideRootScale" 0 false 0))
    (Variables|Default|SetBarrierincineratorRef _returnvalue)
    (CallFunction|SetBarrierincineratorCanDestroyObject false)))

(fn ConstructionScript
  (|CallParentFunction)
  ;[0.03016 0.15 0 0.5] Debug
  (Rendering|Components|TextRender|SetText (Variables|Default|GetComment) (Variables|Default|GetCommentText))
  ;[0.15 0.15 0.15 0.5] Set the exit sign
  (Rendering|SetVisibility (Variables|Default|GetSM_EXIT) (Variables|Default|GetHasExit) false)
  ;[0.15 0.15 0.15 0.5] Set the door lights
  (Rendering|Material|SetColorParameterValueonMaterials (Variables|Default|GetDoorLight1) "EmissiveColor" (Variables|Default|GetColorA))
  ;[0.15 0.15 0.15 0.5] Initialize the Trigglers' collision
  (Collision|SetCollisionResponsetoChannel (Variables|Default|GetAutoCloseTriggerBox) "ECC_Pawn" (select (Variables|Default|GetAutoClose) "ECR_Overlap" "ECR_Ignore"))
  (Collision|SetCollisionResponsetoChannel (Variables|Default|GetAutoOpenTriggerBox) "ECC_Pawn" (select (Variables|Default|GetAutoOpen) "ECR_Overlap" "ECR_Ignore"))
  (Rendering|Material|SetColorParameterValueonMaterials (Variables|Default|GetDoorLight2) "EmissiveColor" (Variables|Default|GetColorA)))

(fn SetBarrierincineratorCanDestroyObject
  (params (CanDestroy :type Boolean))
  (bind _returnvalue (select CanDestroy "QueryOnly" "NoCollision"))
  ;[0.15 0.15 0.15 0.5] Set Barrierincinerator Can Destroy Object
  (bind _barrierincineratorref (Variables|Default|GetBarrierincineratorRef)
    (:then
      (Collision|SetCollisionEnabled (Variables|/Game/SimpleTestChamber/TestElement/Environment/Destory/BP_incinerator.BP_incinerator_C|GetDestoryTriggerBox _barrierincineratorref) _returnvalue)
      (Collision|SetCollisionEnabled (Variables|/Game/SimpleTestChamber/TestElement/Environment/Destory/BP_incinerator.BP_incinerator_C|GetPhyDestoryTriggerBox _barrierincineratorref) _returnvalue)
      (return))
    (:else)))