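; Cube spawner test element that spawns a BP_CubeBase when a button activates it, or optionally at BeginPlay.
; An overlap counter on its trigger box blocks spawning while occupied, flashing the ring's emissive color via timeline to signal refusal or success.
; Each spawn destroys the previous cube and briefly makes the box block the player.
; After the first spawn, a Tick-fed gate optionally respawns the cube when it is destroyed.
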(event OnComponentBeginOverlap(IsTheCubeStillInBoxTriggerbox)
  (params (OverlappedComponent :type Primitive%20Component%20Object%20Reference) (OtherActor :type Actor%20Object%20Reference) (OtherComp :type Primitive%20Component%20Object%20Reference) (OtherBodyIndex :type Integer) (bFromSweep :type Boolean) (SweepResult :type Hit%20Result%20Structure%20%28by%20ref%29))
  (Math|Integer|IncrementInt (Variables|Default|GetBlockNumber)))

(event OnComponentEndOverlap(IsTheCubeStillInBoxTriggerbox)
  (params (OverlappedComponent :type Primitive%20Component%20Object%20Reference) (OtherActor :type Actor%20Object%20Reference) (OtherComp :type Primitive%20Component%20Object%20Reference) (OtherBodyIndex :type Integer))
  (Math|Integer|DecrementInt (Variables|Default|GetBlockNumber)))

(event Custom|SpawnNewCube
  ;[0.15 0.15 0.15 0.5] SpawnNewCube
  (if (> (Variables|Default|GetBlockNumber) 0)
    (Variables|Default|SetColorB "(R=0.229911,G=0.000000,B=0.000000,A=1.000000)")
    (CallFunction|PlayAnimation)
    (else
      (Variables|Default|SetColorB "(R=0.117647,G=0.423529,B=1.000000,A=1.000000)")
      (Utilities|IsValid (Variables|Default|GetCubeRef)
        (:Is%20Valid
          (Class|BPIDestroyCube|DestroyCube(Message) (Variables|Default|GetCubeRef)))
        (:Is%20Not%20Valid
          _))
      (CallFunction|SetBlockPlayer (Variables|Default|GetIsTheCubeStillInBoxTriggerbox) true)
      (bind _returnvalue (Game|SpawnActorfromClass "/Game/SimpleTestChamber/TestElement/Cubes/BP_CubeBase.BP_CubeBase_C" (Transformation|GetWorldTransform (Variables|Default|GetCubeSpwanLocation)) "Undefined" "MultiplyWithRoot" 0 true (Variables|SpawnCube|GetCubeColour) (Variables|SpawnCube|GetChannel) 0))
      (Variables|Default|SetCubeRef _returnvalue)
      (Utilities|FlowControl|Sequence
        (:then_0
          (Utilities|FlowControl|Delay 0.2)
          (CallFunction|SetBlockPlayer (Variables|Default|GetIsTheCubeStillInBoxTriggerbox) false))
        (:then_1
          (CallFunction|PlayAnimation)
          (Utilities|FlowControl|Gate true) ; enters at Open
        )))))

(event Custom|PlayAnimation
  (bind _lerp (Timeline|Activeanimation PlayFromStart)
    (:Update
      (CallFunction|LerponMaterialColor (Variables|Default|GetCubespawenerRin) "EmissiveColor" (Variables|Default|GetColorA) (Variables|Default|GetColorB) _lerp))))

(event EventButtonActive
  (CallFunction|SpawnNewCube))

(event EventBeginPlay
  (if (Variables|Default|GetSpawnOnBeginPlay)
    (CallFunction|SpawnNewCube)))

(event EventTick
  (params (DeltaSeconds :type Float%20%28single-precision%29))
  (Utilities|FlowControl|Gate true
    (:Exit
      (if (Variables|Default|GetSpawnOnCubeDestory)
        (Utilities|IsValid (Variables|Default|GetCubeRef)
          (:Is%20Not%20Valid
            (CallFunction|SpawnNewCube)))))))

(fn ConstructionScript
  (|CallParentFunction)
  (Rendering|Components|TextRender|SetText (Variables|Default|GetComment) (Variables|Default|GetCommentText)))