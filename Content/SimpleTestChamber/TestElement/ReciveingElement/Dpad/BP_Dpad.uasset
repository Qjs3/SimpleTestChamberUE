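; BP_Dpad is a receiving test-chamber element that visually responds to button activation and deactivation.
; ButtonActive plays the Anim timeline and ButtonDeactive reverses it.
; Each timeline update writes the Lerp value to the Alpha and A scalar material parameters on PadD, blending its look between states.
; A PlayAnim call targeting PadD is left unconnected and never runs.
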(event EventButtonActive
  (bind _lerp (Timeline|Anim Play)
    (:Update
      (Rendering|Material|SetScalarParameterValueonMaterials (Variables|Default|GetPadD) "Alpha" _lerp)
      (Rendering|Material|SetScalarParameterValueonMaterials (Variables|Default|GetPadD) "A" _lerp))))

(event EventButtonDeactive
  (bind _lerp (Timeline|Anim Reverse)
    (:Update
      (Rendering|Material|SetScalarParameterValueonMaterials (Variables|Default|GetPadD) "Alpha" _lerp)
      (Rendering|Material|SetScalarParameterValueonMaterials (Variables|Default|GetPadD) "A" _lerp))))

(fn ConstructionScript
  (|CallParentFunction))