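; Base pressure button for test chambers that activates the objects in ActiveObjects while something rests on its trigger box.
; An overlap counter fires activation on the first arrival and deactivation once the box empties.
; A timeline lerps the top's position and emissive color, reversing on release.
; BeginPlay makes the box ignore all channels, then, if PlayerCanActive is set, overlap Pawn and the ActiveCubeType channels.
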(event OnComponentBeginOverlap(Box)
  (params (OverlappedComponent :type Primitive%20Component%20Object%20Reference) (OtherActor :type Actor%20Object%20Reference) (OtherComp :type Primitive%20Component%20Object%20Reference) (OtherBodyIndex :type Integer) (bFromSweep :type Boolean) (SweepResult :type Hit%20Result%20Structure%20%28by%20ref%29))
  ;[0.15 0.15 0.15 0.5] Active
  (Math|Integer|IncrementInt (Variables|Default|GetObjectOnButton)
    (:%20%20
      (if (not (Variables|Default|GetIsActive))
        (Variables|Default|SetIsActive true)
        (Variables|Default|SetOther%20Actor OtherActor)
        (Variables|Default|SetOther%20Comp OtherComp)
        (CallFunction|ActiveLoop (Variables|Default|GetActiveObjects))
        (Default|CallActive)
        ;[0.15 0.15 0.15 0.5] Animation
        (bind _lerp (Timeline|ButtonAimation Play)
          (:Update
            (CallFunction|LerponMaterialColor (Variables|Default|GetButtonTop1) "EmissiveColor" (Variables|Default|GetColorA) (Variables|Default|GetColorB) _lerp)
            (CallFunction|LerponSetLocation (Variables|Default|GetButtonTop) (Variables|Default|GetButtonStartLocation) (Variables|Default|GetButtonEndLocation) _lerp)))))))

(event OnComponentEndOverlap(Box)
  (params (OverlappedComponent :type Primitive%20Component%20Object%20Reference) (OtherActor :type Actor%20Object%20Reference) (OtherComp :type Primitive%20Component%20Object%20Reference) (OtherBodyIndex :type Integer))
  ;[0.15 0.15 0.15 0.5] Deactive
  (if (Variables|Default|GetIsActive)
    (bind _result (Math|Integer|DecrementInt (Variables|Default|GetObjectOnButton))
      (:%20%20
        (if (<= _result 0)
          (Variables|Default|SetIsActive false)
          (Default|CallDeactive)
          (CallFunction|DeactiveLoop (Variables|Default|GetActiveObjects))
          ;[0.15 0.15 0.15 0.5] Animation
          (bind _lerp (Timeline|ButtonAimation Reverse)
            (:Update
              (CallFunction|LerponMaterialColor (Variables|Default|GetButtonTop1) "EmissiveColor" (Variables|Default|GetColorA) (Variables|Default|GetColorB) _lerp)
              (CallFunction|LerponSetLocation (Variables|Default|GetButtonTop) (Variables|Default|GetButtonStartLocation) (Variables|Default|GetButtonEndLocation) _lerp))))))))

(event EventBeginPlay
  ;[0.15 0.15 0.15 0.5] InitializeCollision
  (Collision|SetCollisionResponsetoAllChannels (Variables|Default|GetBox) "ECR_Ignore")
  ;[0.15 0.15 0.15 0.5] set the collison can the button be active
  (if (Variables|Default|GetPlayerCanActive?)
    (Collision|SetCollisionResponsetoChannel (Variables|Default|GetBox) "ECC_Pawn" "ECR_Overlap")
    ;[0.15 0.15 0.15 0.5] set the right kinds of cube to active
    (for _array_element (Variables|Default|GetActiveCubeType)
      (Collision|SetCollisionResponsetoChannel (Variables|Default|GetBox) _array_element "ECR_Overlap"))))

(fn ConstructionScript
  ;[0.15 0.15 0.15 0.5] InitializeColor
  (Rendering|Material|SetColorParameterValueonMaterials (Variables|Default|GetButtonTop) "Base Color" (Variables|Default|GetButtonTopColour)))