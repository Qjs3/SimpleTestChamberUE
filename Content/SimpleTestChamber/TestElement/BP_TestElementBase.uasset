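; Base Blueprint for test chamber elements, providing shared animation, collision and button-messaging helpers.
; PlayAnim runs a timeline at a given speed, lerping component emissive color toward blue, and ReverseAnim plays it backward.
; Helper functions lerp relative location and color, vector or scalar material parameters, and toggle Pawn blocking.
; ActiveLoop and DeactiveLoop send button activate or deactivate messages to each valid actor in an array.
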(event Custom|ReverseAnim
  (params (NewTime :type Float%20%28single-precision%29) (PlaySpeed :type Float%20%28double-precision%29))
  (Variables|Default|SetNew%20Time NewTime)
  (bind _output_get (Variables|Default|SetPlayRate PlaySpeed))
  (Components|Timeline|SetPlayRate (Variables|Default|GetAnimation) _output_get)
  (bind _a (Timeline|Animation Reverse)
    (:Update
      (for _array_element (Variables|Default|GetAnimCompent)
        (CallFunction|LerponMaterialColor :目标 _array_element :ParameterName "EmissiveColor" :B "(R=0.119538,G=0.423268,B=1.000000,A=1.000000)" :Alpha _a)))))

(event Custom|PlayAnim
  (params (NewTime :type Float%20%28single-precision%29) (PlaySpeed :type Float%20%28double-precision%29) (AnimCompent :type Array%20of%20Mesh%20Component%20Object%20References))
  (Variables|Default|SetNew%20Time NewTime)
  (bind _output_get (Variables|Default|SetPlayRate PlaySpeed))
  (Components|Timeline|SetPlayRate (Variables|Default|GetAnimation) _output_get)
  (bind _a (Timeline|Animation Play)
    (:Update
      (for _array_element (Variables|Default|GetAnimCompent)
        (CallFunction|LerponMaterialColor :目标 _array_element :ParameterName "EmissiveColor" :B "(R=0.119538,G=0.423268,B=1.000000,A=1.000000)" :Alpha _a)))))

(fn ConstructionScript)

(fn LerponSetLocation
  (params (目标 :type Scene%20Component%20Object%20Reference) (A :type Vector) (B :type Vector) (Alpha :type Float%20%28single-precision%29))
  (Transformation|SetRelativeLocation 目标 (Math|Vector|Lerp(Vector) A B Alpha) false false)
  (return))

(fn LerponMaterialColor
  (params (目标 :type Mesh%20Component%20Object%20Reference) (ParameterName :type Name) (A :type Linear%20Color%20Structure) (B :type Linear%20Color%20Structure) (Alpha :type Float%20%28single-precision%29))
  (Rendering|Material|SetColorParameterValueonMaterials 目标 ParameterName (Math|Color|Lerp(LinearColor) A B Alpha)))

(fn LerponMaterialVector
  (params (目标 :type Mesh%20Component%20Object%20Reference) (ParameterName :type Name) (A :type Vector) (B :type Vector) (Alpha :type Float%20%28single-precision%29))
  (Rendering|Material|SetVectorParameterValueonMaterials 目标 ParameterName (Math|Vector|Lerp(Vector) A B Alpha)))

(fn LerponMaterialScalar
  (params (目标 :type Mesh%20Component%20Object%20Reference) (ParameterName :type Name) (A :type Float%20%28double-precision%29) (B :type Float%20%28double-precision%29) (Alpha :type Float%20%28double-precision%29))
  (Rendering|Material|SetScalarParameterValueonMaterials 目标 ParameterName (Math|Float|Lerp A B Alpha)))

(fn SetBlockPlayer
  (params (目标 :type Primitive%20Component%20Object%20Reference) (Block :type Boolean))
  (Collision|SetCollisionResponsetoChannel 目标 "ECC_Pawn" (select Block "ECR_Block" "ECR_Ignore")))

(fn ActiveLoop
  (params (Actor :type Array%20of%20Actor%20Object%20References))
  (for _array_element Actor
    (Utilities|IsValid _array_element
      (:Is%20Valid
        (Class|BPIButtonActive|ButtonActive(Message) _array_element))))
  (return))

(fn DeactiveLoop
  (params (Actor :type Array%20of%20Actor%20Object%20References))
  (for _array_element Actor
    (Utilities|IsValid _array_element
      (:Is%20Valid
        (Class|BPIButtonActive|ButtonDeactive(Message) _array_element))))
  (return))