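; BP_CubeBase is a cube actor, apparently a base for test chamber cubes, with configurable colour and animated spawn and destruction.
; The Construction Script applies the colour to the mesh materials and optionally calls Construct, which caches the world scale and plays a timeline scaling up from MinScale.
; BeginPlay sets the collision object type and caches that scale.
; DestroyCube reverses the timeline, then destroys the actor after a short delay.
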(event Custom|Construct
  (Utilities|FlowControl|Sequence
    (:then_0
      (Variables|Default|SetNormalScale (Transformation|GetWorldScale (Variables|Default|GetCubeMesh))))
    (:then_1
      (bind _lerp (Timeline|SpawnAnimation Play)
        (:Update
          (Transformation|SetWorldScale3D (Variables|Default|GetCubeMesh) (Math|Vector|Lerp(Vector) (Variables|Default|GetMinScale) (Variables|Default|GetNormalScale) _lerp)))))))

(event EventBeginPlay
  (Collision|SetCollisionObjectType (Variables|Default|GetCubeMesh) (Variables|Default|GetChannel))
  (Variables|Default|SetNormalScale (Transformation|GetWorldScale (Variables|Default|GetCubeMesh))))

(event EventDestroyCube
  (Utilities|FlowControl|Sequence
    (:then_0
      (bind _lerp (Timeline|SpawnAnimation ReverseFromEnd)
        (:Update
          (Transformation|SetWorldScale3D (Variables|Default|GetCubeMesh) (Math|Vector|Lerp(Vector) (Variables|Default|GetMinScale) (Variables|Default|GetNormalScale) _lerp)))))
    (:then_1
      (Utilities|FlowControl|Delay 0.2)
      (Actor|DestroyActor))))

(fn ConstructionScript
  (Rendering|Material|SetColorParameterValueonMaterials (Variables|Default|GetCubeMesh) "Base Color" (Variables|Default|GetCubeColour))
  (if (Variables|Default|GetPlaySpawnAnim?)
    (CallFunction|Construct)))