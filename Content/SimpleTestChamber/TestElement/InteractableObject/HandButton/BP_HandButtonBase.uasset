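; Base hand button for a test chamber that, on Interact, activates or deactivates its targets according to its button type.
; Normal activates and pops back after a short delay, Switch toggles, and Timer deactivates after a set delay.
; One timeline moves the button top and lerps the ring's emissive color.
; Timer mode rescales that timeline's play rate so the reverse animation acts as a countdown.
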(event Custom|PlayCloseAnim
  ;[0.15 0.15 0.15 0.5] Animation
  (bind _lerpalpha (Timeline|SwitchButtonAnimation Reverse)
    (:Update
      (CallFunction|LerponSetLocation (Variables|Default|GetButtonTop) (Variables|Default|GetButtonStartLocation) (Variables|Default|GetButtonEndLocation) _lerpalpha)
      (CallFunction|LerponMaterialColor (Variables|Default|GethandButtonRin) "EmissiveColor" (Variables|Default|GetColorA) (Variables|Default|GetColorB) _lerpalpha))))

(event Custom|PlayOpenAnim
  ;[0.15 0.15 0.15 0.5] Animation
  (bind _lerpalpha (Timeline|SwitchButtonAnimation Play)
    (:Update
      (CallFunction|LerponSetLocation (Variables|Default|GetButtonTop) (Variables|Default|GetButtonStartLocation) (Variables|Default|GetButtonEndLocation) _lerpalpha)
      (CallFunction|LerponMaterialColor (Variables|Default|GethandButtonRin) "EmissiveColor" (Variables|Default|GetColorA) (Variables|Default|GetColorB) _lerpalpha))))

(event EventInteract
  (bind _delaytime (Variables|Default|GetDelayTime))
  (bind _switchbuttonanimation (Variables|Default|GetSwitchButtonAnimation))
  (bind _returnvalue (- _delaytime 1.0))
  (switch Utilities|FlowControl|Switch|SwitchonE_HandButtonType (Variables|Default|GetButtonType)
    (:NewEnumerator0
      ;[0.15 0.15 0.15 0.5] Normal
      (CallFunction|FActiveButton)
      (Utilities|FlowControl|Delay 0.8)
      (CallFunction|PlayCloseAnim))
    (:NewEnumerator1
      ;[0.15 0.15 0.15 0.5] Switch
      (if (Variables|Default|GetIsActive)
        (CallFunction|FDeactiveButton)
        (else
          (CallFunction|FActiveButton))))
    (:NewEnumerator2
      ;[0.15 0.15 0.15 0.5] Timer
      (CallFunction|FActiveButton)
      (Utilities|FlowControl|Delay 1.0)
      (Utilities|FlowControl|Sequence
        (:then_0
          (Components|Timeline|SetPlaybackPosition _switchbuttonanimation 1.0 false true)
          (Components|Timeline|SetPlayRate _switchbuttonanimation (/ 1.0 _returnvalue))
          (CallFunction|PlayCloseAnim)
          (Utilities|FlowControl|RetriggerableDelay _returnvalue)
          (Components|Timeline|SetPlayRate (Variables|Default|GetSwitchButtonAnimation) 1.0)
          (CallFunction|FDeactiveButton))
        (:then_1
          (Utilities|FlowControl|RetriggerableDelay (Variables|Default|GetDelayTime))
          (Components|Timeline|SetPlayRate _switchbuttonanimation 1.0)
          (CallFunction|FDeactiveButton))))))

(event EventBeginPlay)

(fn ConstructionScript
  (|CallParentFunction)
  (Rendering|Components|TextRender|SetText (Variables|Default|GetComment) (Variables|Default|GetCommentText))
  (Components|Timeline|SetPlayRate (Variables|Default|GetSwitchButtonAnimation) 0.7))

(fn FActiveButton
  (Default|CallActive)
  (CallFunction|ActiveLoop (Variables|Default|GetActiveTarget))
  (CallFunction|PlayOpenAnim)
  (Variables|Default|SetIsActive true)
  (return))

(fn FDeactiveButton
  (Default|CallDeactive)
  (CallFunction|DeactiveLoop (Variables|Default|GetActiveTarget))
  (CallFunction|PlayCloseAnim)
  (Variables|Default|SetIsActive false)
  (return))